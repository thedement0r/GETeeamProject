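; BP_Dial is a single ten-digit dial of a combination lock minigame, starting at a random digit on BeginPlay.
; RotateDial plays a click and uses a timeline to turn the mesh one digit step, ignoring input until it finishes.
; The resulting yaw wraps after a full turn and is converted to Number, then LocREF is told to check the lock.
; An arrow widget is initialized with a reference to the dial.
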(event Custom|FindNunber
  (Variables|Default|SetNumber (Math|Float|Truncate (/ (Variables|Default|GetDialRotation) 36.0))))

(event Custom|RotateDial
  (if (Variables|Default|GetcanRotate)
    (Variables|Default|SetcanRotate false)
    (Audio|PlaySound2D "/Game/Minigame/CombinationLockClick.CombinationLockClick" 1.0 1.0 0.0 0 0)
    (bind _alpha (Timeline|DialRotation_TL PlayFromStart)
      (:Update
        (Transformation|SetRelativeRotation (Variables|Default|GetSM_Dial) (Math|Rotator|MakeRotator 0.0 0.0 (+ (Variables|Default|GetDialRotation) (Math|Float|Lerp 0.0 36.0 _alpha))) false false))
      (:Finished
        (Variables|Default|SetDialRotation (+ (Variables|Default|GetDialRotation) (Math|Float|Lerp 0.0 36.0 _alpha)))
        (if (>= (Variables|Default|GetDialRotation) 3.6e+02)
          (Variables|Default|SetDialRotation 0.0)
          (Transformation|SetRelativeRotation (Variables|Default|GetSM_Dial) "0, 0, 0" false false))
        (CallFunction|FindNunber)
        (Default|CheckEveryTurn (Variables|Default|GetLoc%20REF))
        (Variables|Default|SetcanRotate true)))))

(event EventBeginPlay
  (bind _aswb_arrow (Utilities|Casting|CastToWB_Arrow (UserInterface|GetUserWidgetObject (Variables|Default|GetArrow))))
  (Default|Initialize _aswb_arrow self)
  (CallFunction|SetRndNum))

(fn ConstructionScript)

(fn SetRndNum
  (bind _output_get (LocalVariables|SetLocalRotation (* (Math|Random|RandomIntegerinRange 0 9) 36.0)))
  (Transformation|SetRelativeRotation (Variables|Default|GetSM_Dial) (Math|Rotator|MakeRotator 0.0 0.0 _output_get) false false)
  (Variables|Default|SetDialRotation (LocalVariables|GetLocalRotation))
  (CallFunction|FindNunber))