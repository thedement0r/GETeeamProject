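; AC_Skills is a skill tree component that tracks available skill points and a map of assigned skills to their ranks.
; AssignSkill checks prerequisites, tier limit and points, then raises the rank, spends a point and fires OnSkillsUpdated.
; A skill's valid Ability is added to player character 0's AC_Abilities, regardless of the component's owner.
; UnassignSkill only lowers the rank, without refunding points, removing abilities or firing the update.
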(event EventBeginPlay)

(event EventTick
  (params (DeltaSeconds :type Float%20%28single-precision%29)))

(fn AwardSkillPoint
  (params (SkillPoints :type Integer))
  (Variables|Default|SetSkillPointsAvailable (+ SkillPoints (Variables|Default|GetSkillPointsAvailable))))

(fn SpendSkillPoint
  (params (Amount :type Integer))
  (if (CallFunction|QuerySkillPoints Amount)
    (Variables|Default|SetSkillPointsAvailable (- (Variables|Default|GetSkillPointsAvailable) Amount))))

(fn QuerySkillPoints
  (params (Query :type Integer))
  (return (>= (Variables|Default|GetSkillPointsAvailable) Query)))

(fn AssignSkill
  (params (Skill :type DA%20Skill%20Object%20Reference%20%28by%20ref%29))
  (bind _skillsassigned (Variables|Default|GetSkillsAssigned))
  (bind (_value _returnvalue) (Utilities|Map|Find _skillsassigned Skill))
  (if (Math|Boolean|ANDBoolean (Default|ArePrerequisiteMet Skill self) (<= (+ (.Value (Utilities|Map|Find (Variables|Default|GetSkillsAssigned) Skill)) 1) (Default|GetNumberOfTiers Skill)) (CallFunction|QuerySkillPoints 1))
    (Utilities|Map|Add (Variables|Default|GetSkillsAssigned) Skill (Math|Integer|SelectInt (+ _value 1) 1 _returnvalue))
    (CallFunction|SpendSkillPoint 1)
    (Default|CallOnSkillsUpdated)
    (bind _ability (Variables|/Game/Skilltree/Data/DA_Skill.DA_Skill_C|GetAbility Skill)
      (:then
        (Default|AddAbility (Actor|GetComponentbyClass (Game|GetPlayerCharacter 0) "/Game/Abilities/AC_Abilities.AC_Abilities_C") _ability))
      (:else))))

(fn UnassignSkill
  (params (Skill :type DA%20Skill%20Object%20Reference%20%28by%20ref%29))
  (if (> (.Rank (CallFunction|QuerySkill Skill)) 0)
    (Utilities|Map|Add (Variables|Default|GetSkillsAssigned) Skill (- (.Value (Utilities|Map|Find (Variables|Default|GetSkillsAssigned) Skill)) 1))))

(fn QuerySkill
  (params (Skill :type DA%20Skill%20Object%20Reference))
  (bind _skillsassigned (Variables|Default|GetSkillsAssigned))
  (bind (_value _returnvalue) (Utilities|Map|Find _skillsassigned Skill))
  (return _value _returnvalue Skill))