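; Health power-up pickup that restores a fixed amount of HP to a BP_Character that overlaps it.
; On pickup it calls IncreaseHP on the character's BPPlayerStats and attaches a Niagara healing effect to the mesh's spine socket.
; It then hides itself and reappears after a short delay, using the hidden flag to ignore overlaps while it is on cooldown.
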(event EventBeginPlay
  (|CallParentFunction) ; This node is disabled and will not be called.\nDrag off pins to build functionality.
)

(event Collision|EventActorBeginOverlap
  (params (OtherActor :type Actor%20Object%20Reference))
  (bind _asbp_character (Utilities|Casting|CastToBP_Character OtherActor))
  (if (not (Variables|Default|GetbHidden))
    (Default|IncreaseHP (Variables|/Game/Blueprints/BP_Character.BP_Character_C|GetBP_PlayerStats _asbp_character) 2e+01)
    (Niagara|SpawnSystemAttached "/Game/Assets/sA_PickupSet_1/Fx/NiagaraSystems/NS_Healing_1.NS_Healing_1" (Variables|/Script/Engine.Character|GetMesh _asbp_character) "spine_03" "0, 0, 0" "-90.000000,0.000000,0.000000" "KeepRelativeOffset" true)
    (Rendering|SetActorHiddenInGame true)
    (Utilities|FlowControl|Delay 5.0)
    (Rendering|SetActorHiddenInGame false)))

(event EventTick
  (params (DeltaSeconds :type Float%20%28single-precision%29))
  (|CallParentFunction DeltaSeconds) ; This node is disabled and will not be called.\nDrag off pins to build functionality.
)

(fn ConstructionScript
  (|CallParentFunction))