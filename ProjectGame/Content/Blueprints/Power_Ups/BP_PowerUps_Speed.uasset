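; Speed power-up pickup that grants a speed boost to the player character on overlap.
; When a BP_Character overlaps it while visible, it calls ActivateSpeedBoost on that character and hides itself.
; After a five-second delay it reappears, with the hidden flag doubling as the guard against pickups during the respawn window.
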(event EventBeginPlay
  (|CallParentFunction) ; This node is disabled and will not be called.\nDrag off pins to build functionality.
)

(event Collision|EventActorBeginOverlap
  (params (OtherActor :type Actor%20Object%20Reference))
  (bind _asbp_character (Utilities|Casting|CastToBP_Character OtherActor))
  (if (not (Variables|Default|GetbHidden))
    (Default|ActivateSpeedBoost _asbp_character)
    (Rendering|SetActorHiddenInGame true)
    (Utilities|FlowControl|Delay 5.0)
    (Rendering|SetActorHiddenInGame false)))

(event EventTick
  (params (DeltaSeconds :type Float%20%28single-precision%29))
  (|CallParentFunction DeltaSeconds) ; This node is disabled and will not be called.\nDrag off pins to build functionality.
)

(fn ConstructionScript
  (|CallParentFunction))