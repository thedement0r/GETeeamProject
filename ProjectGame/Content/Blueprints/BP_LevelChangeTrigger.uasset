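; BP_LevelChangeTrigger is a trigger volume that saves the game and moves the player to another level.
; When a BP_Character overlaps its box, it binds to the GI_Selections game-saved event and requests a save without a message flag.
; Once the save completes, it shows the WB_LoadingScreen widget, waits briefly, then opens the configured level by object reference.
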(event OnComponentBeginOverlap(Box)
  (params (OverlappedComponent :type Primitive%20Component%20Object%20Reference) (OtherActor :type Actor%20Object%20Reference) (OtherComp :type Primitive%20Component%20Object%20Reference) (OtherBodyIndex :type Integer) (bFromSweep :type Boolean) (SweepResult :type Hit%20Result%20Structure%20%28by%20ref%29))
  (Utilities|Casting|CastToBP_Character OtherActor)
  (bind _asgi_selections (Utilities|Casting|CastToGI_Selections (Game|GetGameInstance)))
  (EventDispatchers|BindEventtoGameSaved _asgi_selections (delegate Custom|SaveCompleted))
  (Class|BPPersistence|RequestSave(Message) _asgi_selections false))

(event Custom|SaveCompleted
  (params (SaveGameRef :type BP%20Save%20Game%20Object%20Reference))
  (bind _returnvalue (UserInterface|CreateWidget "/Game/MainMenu/WB_LoadingScreen.WB_LoadingScreen_C"))
  (UserInterface|Viewport|AddtoViewport _returnvalue 0)
  (Utilities|FlowControl|Delay 1.0)
  (Game|OpenLevel(byObjectReference) (Variables|Default|GetLevel)))

(fn ConstructionScript)