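; Stats component for player, dummy and AI owners that tracks HP, and XP and level with player HUD updates.
; BeginPlay casts the owner to set CharacterType, which selects the health bar DecreaseHP updates; DecreaseHP also reports death.
; Filling XP raises the level and XP cap, resets XP and awards an AC_Skills point.
; Tick sums Health skill bonuses, but the IncreaseMaxHP call that would apply them is disconnected.
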(event EventBeginPlay
  (Utilities|FlowControl|DelayUntilNextTick)
  (bind _asbp_character (Utilities|Casting|CastToBP_Character (Components|GetOwner))
    (:then
      (Variables|Default|SetPlayer%20Character%20Bp _asbp_character)
      (Variables|Default|SetisPlayer true)
      (Variables|Default|SetCharacter%20Type "NewEnumerator0")
      (bind _returnvalue (Game|GetCurrentLevelName true))
      (if (not (Utilities|Set|Contains (Variables|/Game/Blueprints/BP_Character.BP_Character_C|GetNonHUDLevels (Variables|Default|GetPlayer%20Character%20Bp)) _returnvalue))
        (Progress|SetPercent (Utilities|Select :Index (Variables|Default|GetCharacter%20Type) :NewEnumerator0 (Variables|/Game/UI/WB_HUD.WB_HUD_C|GetHPBar (Variables|/Game/Blueprints/BP_Character.BP_Character_C|GetHUD%20Widget (Variables|Default|GetPlayer%20Character%20Bp))) :NewEnumerator1 (Variables|/Game/UI/WB_DummyHealthBar.WB_DummyHealthBar_C|GetHealthBar (Variables|/Game/Blueprints/BP_Dummy.BP_Dummy_C|GetHealthBar%20UI (Variables|Default|GetDummy%20BP))) :NewEnumerator2 (Variables|/Game/UI/WB_DummyHealthBar.WB_DummyHealthBar_C|GetHealthBar (Variables|/Game/AI/BP_AI.BP_AI_C|GetHealthBar%20UI (Variables|Default|GetAI%20BP)))) (/ (Variables|Health|GetCurrentHP) (Variables|Health|GetMaxHP)) :!label _label)))
    (:CastFailed
      (bind _asbp_dummy (Utilities|Casting|CastToBP_Dummy (Components|GetOwner))
        (:then
          (Variables|Default|SetDummy%20BP _asbp_dummy)
          (Variables|Default|SetisPlayer false)
          (Variables|Default|SetCharacter%20Type "NewEnumerator1")
          (goto _label))
        (:CastFailed
          (bind _asbp_ai (Utilities|Casting|CastToBP_AI (Components|GetOwner)))
          (Variables|Default|SetAI%20BP _asbp_ai)
          (Variables|Default|SetCharacter%20Type "NewEnumerator2"))))))

(event EventTick
  (params (DeltaSeconds :type Float%20%28single-precision%29))
  (bind _increment (Health|CalculateIncrement)))

(fn DecreaseHP
  (params (Decreased%20HP :type Float%20%28double-precision%29))
  (bind _player_character_bp (Variables|Default|GetPlayer%20Character%20Bp))
  (bind _hud_widget (Variables|/Game/Blueprints/BP_Character.BP_Character_C|GetHUD%20Widget _player_character_bp))
  (if (not (<= (Variables|Health|GetCurrentHP) 0.0))
    (bind _output_get (Variables|Health|SetCurrentHP (- (Variables|Health|GetCurrentHP) Decreased%20HP)))
    (Rendering|Components|TextRender|SetText (Variables|/Game/UI/WB_HUD.WB_HUD_C|GetTXT_HealthPoints _hud_widget) (Utilities|Text|FormatText "{Current HP} / {Max HP}" (Variables|Health|GetCurrentHP) (Variables|Health|GetMaxHP)))
    (Progress|SetPercent (Utilities|Select :Index (Variables|Default|GetCharacter%20Type) :NewEnumerator0 (Variables|/Game/UI/WB_HUD.WB_HUD_C|GetHPBar _hud_widget) :NewEnumerator1 (Variables|/Game/UI/WB_DummyHealthBar.WB_DummyHealthBar_C|GetHealthBar (Variables|/Game/Blueprints/BP_Dummy.BP_Dummy_C|GetHealthBar%20UI (Variables|Default|GetDummy%20BP))) :NewEnumerator2 (Variables|/Game/UI/WB_DummyHealthBar.WB_DummyHealthBar_C|GetHealthBar (Variables|/Game/AI/BP_AI.BP_AI_C|GetHealthBar%20UI (Variables|Default|GetAI%20BP)))) (/ _output_get (Variables|Health|GetMaxHP)))
    (if (<= (Variables|Health|GetCurrentHP) 0.0)
      _
      (else
        (return false))))
  (return true))

(fn IncreaseMaxHP
  (params (Incremention :type Float%20%28double-precision%29))
  (bind _currenthp (Variables|Health|GetCurrentHP))
  (bind _player_character_bp (Variables|Default|GetPlayer%20Character%20Bp))
  (bind _hud_widget (Variables|/Game/Blueprints/BP_Character.BP_Character_C|GetHUD%20Widget _player_character_bp))
  (bind _output_get (Variables|Health|SetMaxHP (+ 1e+02 Incremention)))
  (Rendering|Components|TextRender|SetText (Variables|/Game/UI/WB_HUD.WB_HUD_C|GetTXT_HealthPoints _hud_widget) (Utilities|Text|FormatText "{Current HP} / {Max HP}" _currenthp _output_get))
  (Progress|SetPercent (Variables|/Game/UI/WB_HUD.WB_HUD_C|GetHPBar _hud_widget) (/ _currenthp (Variables|Health|GetMaxHP))))

(fn IncreaseHP
  (params (Added%20Health :type Float%20%28double-precision%29))
  (bind _maxhp (Variables|Health|GetMaxHP))
  (bind _maxhp_2 (Variables|Health|GetMaxHP))
  (Variables|Health|SetCurrentHP (+ (Variables|Health|GetCurrentHP) Added%20Health))
  (if (> (Variables|Health|GetCurrentHP) (Variables|Health|GetMaxHP))
    (bind _output_get (Variables|Health|SetCurrentHP _maxhp))
    (Rendering|Components|TextRender|SetText (Variables|/Game/UI/WB_HUD.WB_HUD_C|GetTXT_HealthPoints (Variables|/Game/Blueprints/BP_Character.BP_Character_C|GetHUD%20Widget (Variables|Default|GetPlayer%20Character%20Bp))) (Utilities|Text|FormatText "{Current HP} / {Max HP}" _output_get _maxhp))
    (else
      (Rendering|Components|TextRender|SetText (Variables|/Game/UI/WB_HUD.WB_HUD_C|GetTXT_HealthPoints (Variables|/Game/Blueprints/BP_Character.BP_Character_C|GetHUD%20Widget (Variables|Default|GetPlayer%20Character%20Bp))) (Utilities|Text|FormatText "{Current HP} / {Max HP}" (Variables|Health|GetCurrentHP) _maxhp_2))))
  (Progress|SetPercent (Variables|/Game/UI/WB_HUD.WB_HUD_C|GetHPBar (Variables|/Game/Blueprints/BP_Character.BP_Character_C|GetHUD%20Widget (Variables|Default|GetPlayer%20Character%20Bp))) (/ (Variables|Health|GetCurrentHP) _maxhp_2)))

(fn IncreaseXP
  (params (Added%20XP :type Float%20%28double-precision%29))
  (Variables|XP|SetCurrentXP (+ (Variables|XP|GetCurrentXP) Added%20XP))
  (if (>= (Variables|XP|GetCurrentXP) (Variables|XP|GetMaxXP))
    (LevelXP|IncreaseLevel 1)
    (Default|AwardSkillPoint (Actor|GetComponentbyClass (Game|GetPlayerCharacter 0) "/Game/Skilltree/AC_Skills.AC_Skills_C") 1))
  (Progress|SetPercent (Variables|/Game/UI/WB_HUD.WB_HUD_C|GetXPBar (Variables|/Game/Blueprints/BP_Character.BP_Character_C|GetHUD%20Widget (Variables|Default|GetPlayer%20Character%20Bp))) (/ (Variables|XP|GetCurrentXP) (Variables|XP|GetMaxXP)))
  (Rendering|Components|TextRender|SetText (Variables|/Game/UI/WB_HUD.WB_HUD_C|GetXPText (Variables|/Game/Blueprints/BP_Character.BP_Character_C|GetHUD%20Widget (Variables|Default|GetPlayer%20Character%20Bp))) (Utilities|Text|FormatText "{Current XP} / {Max XP}" (Variables|XP|GetCurrentXP) (Variables|XP|GetMaxXP))))

(fn IncreaseLevel
  (params (Added%20Level :type Integer))
  (Variables|XP|SetLevel (+ (Variables|XP|GetLevel) Added%20Level))
  (Variables|XP|SetMaxXP (+ (Variables|XP|GetMaxXP) 1.5e+02))
  (Variables|XP|SetCurrentXP 0.0)
  (Rendering|Components|TextRender|SetText (Variables|/Game/UI/WB_HUD.WB_HUD_C|GetLevelText (Variables|/Game/Blueprints/BP_Character.BP_Character_C|GetHUD%20Widget (Variables|Default|GetPlayer%20Character%20Bp))) (Utilities|Text|ToText(Integer) (Variables|XP|GetLevel))))

(fn CalculateIncrement
  (bind _returnvalue (Game|GetPlayerCharacter 0))
  (bind _returnvalue_2 (Actor|GetComponentbyClass _returnvalue "/Game/Skilltree/AC_Skills.AC_Skills_C"))
  (bind (_rank _returnvalue_3 _skillout) (Default|QuerySkill _returnvalue_2 "/Game/Skilltree/Data/Health2.Health2"))
  (bind (_rank_2 _returnvalue_4 _skillout_2) (Default|QuerySkill _returnvalue_2 "/Game/Skilltree/Data/Health3.Health3"))
  (bind (_rank_3 _returnvalue_5 _skillout_3) (Default|QuerySkill _returnvalue_2 "/Game/Skilltree/Data/Health1.Health1"))
  (bind _values (Variables|/Game/Skilltree/Data/DA_Skill.DA_Skill_C|GetValues _skillout_2))
  (bind _values_2 (Variables|/Game/Skilltree/Data/DA_Skill.DA_Skill_C|GetValues _skillout_3))
  (bind _values_3 (Variables|/Game/Skilltree/Data/DA_Skill.DA_Skill_C|GetValues _skillout))
  (bind (_value _returnvalue_6) (Utilities|Map|Find _values_3 _rank))
  (bind (_value_2 _returnvalue_7) (Utilities|Map|Find _values _rank_2))
  (bind (_value_3 _returnvalue_8) (Utilities|Map|Find _values_2 _rank_3))
  (return (+ 0.0 (Math|Float|SelectFloat _value_3 0.0 _returnvalue_8) (Math|Float|SelectFloat _value 0.0 _returnvalue_6) (Math|Float|SelectFloat _value_2 0.0 _returnvalue_7))))