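; BP_Bounds is a playable-area volume that kills a BP_Character who stays outside it too long.
; Leaving BoundsTriger sets OutOfBounds, shows a WB_OutOfBounds warning and starts a short delay.
; If the flag is still set afterwards, it passes the character's full current HP to DecreaseHP and, on a true result, shows a death message and calls Die.
; Re-entering clears the flag and removes the widget.
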(event OnComponentEndOverlap(BoundsTriger)
  (params (OverlappedComponent :type Primitive%20Component%20Object%20Reference) (OtherActor :type Actor%20Object%20Reference) (OtherComp :type Primitive%20Component%20Object%20Reference) (OtherBodyIndex :type Integer))
  (bind _asbp_character (Utilities|Casting|CastToBP_Character OtherActor))
  (Variables|Default|SetOutOfBounds true)
  (Utilities|IsValid (Variables|Default|GetWidgetRef)
    (:Is%20Not%20Valid
      (bind _returnvalue (UserInterface|CreateWidget "/Game/UI/WB_OutOfBounds.WB_OutOfBounds_C"))
      (bind _output_get (Variables|Default|SetWidgetRef _returnvalue))
      (UserInterface|Viewport|AddtoViewport _output_get 0)
      (Utilities|FlowControl|Delay 5.0)
      (if (Variables|Default|GetOutOfBounds)
        (bind _isplayerdead (Default|DecreaseHP (Variables|/Game/Blueprints/BP_Character.BP_Character_C|GetBP_PlayerStats _asbp_character) (Variables|/Game/Blueprints/BP_PlayerStats.BP_PlayerStats_C|GetCurrentHP (Variables|/Game/Blueprints/BP_Character.BP_Character_C|GetBP_PlayerStats _asbp_character))))
        (if _isplayerdead
          (Rendering|Components|TextRender|SetText (Variables|/Game/UI/WB_OutOfBounds.WB_OutOfBounds_C|GetTextBlock (Variables|Default|GetWidgetRef)) "YOU'RE DEAD")
          (Default|Die _asbp_character))))))

(event OnComponentBeginOverlap(BoundsTriger)
  (params (OverlappedComponent :type Primitive%20Component%20Object%20Reference) (OtherActor :type Actor%20Object%20Reference) (OtherComp :type Primitive%20Component%20Object%20Reference) (OtherBodyIndex :type Integer) (bFromSweep :type Boolean) (SweepResult :type Hit%20Result%20Structure%20%28by%20ref%29))
  (Utilities|Casting|CastToBP_Character OtherActor)
  (Variables|Default|SetOutOfBounds false)
  (bind _widgetref (Variables|Default|GetWidgetRef)
    (:then
      (Widget|RemovefromParent _widgetref)
      (Variables|Default|SetWidgetRef 0))
    (:else)))

(event EventBeginPlay)

(event Collision|EventActorBeginOverlap
  (params (OtherActor :type Actor%20Object%20Reference)))

(event EventTick
  (params (DeltaSeconds :type Float%20%28single-precision%29)))

(fn ConstructionScript)