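; BP_Dummy is a character that serves as a target for player attacks and stealth back assassinations.
; Damage plays a random hit montage, launches it along the player's forward vector and lowers HP through BPPlayerStats, ragdolling when DecreaseHP returns true.
; An overlap radius toggles the assassinate prompt, which turns with the health bar toward the camera each tick.
; StealthBackAssassin plays the victim montage, triggers a delayed ragdoll and returns the attacker's reference location and rotation.
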(event OnComponentBeginOverlap(AssassinationRadius)
  (params (OverlappedComponent :type Primitive%20Component%20Object%20Reference) (OtherActor :type Actor%20Object%20Reference) (OtherComp :type Primitive%20Component%20Object%20Reference) (OtherBodyIndex :type Integer) (bFromSweep :type Boolean) (SweepResult :type Hit%20Result%20Structure%20%28by%20ref%29))
  (Utilities|Casting|CastToBP_Character OtherActor)
  (Rendering|SetVisibility (Variables|Default|GetAssassinate%20Widget) true false))

(event OnComponentEndOverlap(AssassinationRadius)
  (params (OverlappedComponent :type Primitive%20Component%20Object%20Reference) (OtherActor :type Actor%20Object%20Reference) (OtherComp :type Primitive%20Component%20Object%20Reference) (OtherBodyIndex :type Integer))
  (Utilities|Casting|CastToBP_Character OtherActor)
  (Rendering|SetVisibility (Variables|Default|GetAssassinate%20Widget) false false))

(event Custom|Ragdoll
  ;[1 1 1] Ragdoll
  (Utilities|FlowControl|Delay 2.5)
  (Physics|SetSimulatePhysics (Variables|Character|GetMesh) true))

(event EventTick
  (params (DeltaSeconds :type Float%20%28single-precision%29))
  (Transformation|SetWorldRotation (Variables|Default|GetAssassinate%20Widget) (Math|Rotator|FindLookatRotation (Transformation|GetWorldLocation (Variables|Default|GetAssassinate%20Widget)) (Transformation|GetWorldLocation (Variables|/Script/Engine.PlayerCameraManager|GetTransformComponent (Game|GetPlayerCameraManager 0)))) false false))

(event EventBeginPlay
  (bind _aswb_dummy_health_bar (Utilities|Casting|CastToWB_DummyHealthBar (UserInterface|GetWidget (Variables|Default|GetHealth%20Bar%20Widget))))
  (Variables|Default|SetHealthBar%20UI _aswb_dummy_health_bar))

(event Game|Damage|EventAnyDamage
  (params (Damage :type Float%20%28single-precision%29) (DamageType :type Damage%20Type%20Object%20Reference) (InstigatedBy :type Controller%20Object%20Reference) (DamageCauser :type Actor%20Object%20Reference))
  (Animation|PlayAnimMontage (Utilities|Array|Get(acopy) (Variables|Default|GethitAnims) (Math|Random|RandomIntegerinRange 0 (- (Utilities|Array|Length (Variables|Default|GethitAnims)) 1))) 1.0 "None")
  (bind _asbp_character (Utilities|Casting|CastToBP_Character (Game|GetPlayerCharacter 0)))
  (Character|LaunchCharacter (* (Math|Vector|GetForwardVector (Transformation|GetActorRotation _asbp_character)) 7e+02) false false)
  (bind _isplayerdead (Default|DecreaseHP (Variables|Default|GetBP_PlayerStats) Damage))
  (if _isplayerdead
    (Physics|SetSimulatePhysics (Variables|Character|GetMesh) true)))

(fn ConstructionScript)

(fn StealthBackAssassin
  (Animation|PlayAnimMontage "/Game/Animations/Assassination/Paired_Knife_Stealth_KidneyAndNeck_Vic_Montage.Paired_Knife_Stealth_KidneyAndNeck_Vic_Montage" 1.0 "None")
  (CallFunction|Ragdoll)
  (Rendering|SetVisibility (Variables|Default|GetAssassinate%20Widget) false false)
  (return (Transformation|GetWorldLocation (Variables|Default|GetAssassin%20REF)) (Transformation|GetActorRotation)))