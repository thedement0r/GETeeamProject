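; Player combat component on BP_Character that runs a four-step sword-and-kick montage combo from the attack input.
; Input during an attack is buffered, and SwordAttackCombo either plays the next AttackIndex step or resets the combo.
; A looping timer sphere-sweeps between sword points with a hit cooldown, while SphereTrace covers stab and kick.
; Hits on "abc"-tagged actors deal PlayerDamage plus bonuses from three AC_Skills sword skills.
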(event Custom|Sword%20Attack
  ;[1 1 1] Combo system
  (if (Variables|Default|GetisAttacking)
    (Variables|Default|SetsaveAttack true)
    (else
      (Variables|Default|SetisAttacking true)
      (switch int (Variables|Default|GetAttackIndex)
        (:0
          (CallFunction|Attack1))
        (:1
          (CallFunction|Attack2))
        (:2
          (CallFunction|Attack3))
        (:3
          (CallFunction|Attack4))))))

(event Custom|Sword%20Attack%20Combo
  ;[1 1 1] Combo system
  (if (Variables|Default|GetsaveAttack)
    (Variables|Default|SetsaveAttack false)
    (switch int (Variables|Default|GetAttackIndex)
      (:0
        (CallFunction|Attack1))
      (:1
        (CallFunction|Attack2))
      (:2
        (CallFunction|Attack3))
      (:3
        (CallFunction|Attack4)))
    (else
      (CallFunction|StopCombo))))

(event Custom|Start%20Sword%20Trace
  ;[1 1 1] Sword Trace
  (bind _returnvalue (Utilities|Time|SetTimerbyEvent (delegate Custom|Sword%20Trace%20Loop) 0.01 true))
  (Variables|Default|SetSwordTraceLoop _returnvalue))

(event Custom|Sword%20Trace%20Loop
  ;[1 1 1] Sword Trace
  (bind (_outhit _returnvalue) (Collision|SphereTraceByChannel (Transformation|GetWorldLocation (Variables|/Game/Blueprints/BP_Character.BP_Character_C|GetSword%20Top%20Point (Variables|Default|GetCharacterBP))) (Transformation|GetWorldLocation (Variables|/Game/Blueprints/BP_Character.BP_Character_C|GetSword%20Bottom%20Point (Variables|Default|GetCharacterBP))) 12.0 "TraceTypeQuery1" false 0 "None" true "(R=1.000000,G=0.000000,B=0.000000,A=1.000000)" "(R=0.000000,G=1.000000,B=0.000000,A=1.000000)" 0.2))
  (if _returnvalue
    (if (Actor|ActorHasTag (.HitActor (Collision|BreakHitResult _outhit)) "abc")
      (Utilities|FlowControl|DoOnce false :!label _label
        (:Completed
          (bind _damage (CallFunction|CalculateDamage))
          (Game|Damage|ApplyDamage (.HitActor (Collision|BreakHitResult _outhit)) _damage 0 0)
          (Utilities|FlowControl|Delay 0.5)
          (goto _label Reset))))))

(event Custom|Stop%20Sword%20Trace
  ;[1 1 1] Sword Trace
  (Utilities|Time|ClearandInvalidateTimerbyHandle (Variables|Default|GetSwordTraceLoop)))

(event Custom|Sphere%20Trace
  (bind _characterbp (Variables|Default|GetCharacterBP))
  (bind _sphere_trace (Variables|/Game/Blueprints/BP_Character.BP_Character_C|GetSphere%20Trace _characterbp))
  (bind _returnvalue (Transformation|GetWorldLocation _sphere_trace))
  ;[1 1 1] Sphere Trace for stab+kick
  (bind (_outhit _returnvalue_2) (Collision|SphereTraceByChannel _returnvalue _returnvalue 25.0 "TraceTypeQuery1" false 0 "None"))
  (if _returnvalue_2
    (if (Actor|ActorHasTag (.HitActor (Collision|BreakHitResult _outhit)) "abc")
      (bind _damage (CallFunction|CalculateDamage))
      (Game|Damage|ApplyDamage (.HitActor (Collision|BreakHitResult _outhit)) _damage 0 0))))

(event Custom|Stop%20Combo
  ;[1 1 1] Combo system
  (Variables|Default|SetisAttacking false)
  (Variables|Default|SetAttackIndex 0))

(event Custom|Attack%204
  ;[1 1 1] Combo system
  (Utilities|FlowControl|DoOnce false :!label _label
    (:Completed
      (Utilities|FlowControl|Delay 0.1)
      (Animation|Montage|PlayMontage (Variables|Default|GetCharacter%20Mesh) "/Game/Animations/SwordAttack/Attack3_Montage.Attack3_Montage"
        (:then
          (Variables|Default|SetAttackIndex 4)
          (goto _label Reset))))))

(event Custom|Attack%201
  ;[1 1 1] Combo system
  (Utilities|FlowControl|DoOnce false :!label _label
    (:Completed
      (Utilities|FlowControl|Delay 0.1)
      (Animation|Montage|PlayMontage (Variables|Default|GetCharacter%20Mesh) "/Game/Animations/SwordAttack/Attack1_Montage.Attack1_Montage"
        (:then
          (Variables|Default|SetAttackIndex 1)
          (goto _label Reset))))))

(event Custom|Attack2
  ;[1 1 1] Combo system
  (Utilities|FlowControl|DoOnce false :!label _label
    (:Completed
      (Utilities|FlowControl|Delay 0.1)
      (Animation|Montage|PlayMontage (Variables|Default|GetCharacter%20Mesh) "/Game/Animations/SwordAttack/Attack2_Montage.Attack2_Montage"
        (:then
          (Variables|Default|SetAttackIndex 2)
          (goto _label Reset))))))

(event Custom|Attack%203
  ;[1 1 1] Combo system
  (Utilities|FlowControl|DoOnce false :!label _label
    (:Completed
      (Utilities|FlowControl|Delay 0.1)
      (Animation|Montage|PlayMontage (Variables|Default|GetCharacter%20Mesh) "/Game/Animations/SwordAttack/Kick_Montage.Kick_Montage"
        (:then
          (Variables|Default|SetAttackIndex 3)
          (goto _label Reset))))))

(event Input|EnhancedActionEvents|EnhancedInputActionIA_Attack
  (params (ActionValue :type Boolean) (ElapsedSeconds :type Float%20%28double-precision%29) (TriggeredSeconds :type Float%20%28double-precision%29) (InputAction :type Input%20Action%20Object%20Reference :default "/Game/Animations/SwordAttack/InputAttack/IA_Attack.IA_Attack"))
  ;[1 1 1] Combo system
  (:Started
    (if (Variables|Default|GetcanAttack)
      (CallFunction|SwordAttack))))

(event EventBeginPlay
  (bind _asbp_character (Utilities|Casting|CastToBP_Character (Components|GetOwner)))
  (Variables|Default|SetCharacterBP _asbp_character)
  (Variables|Default|SetCharacter%20Mesh (Variables|/Script/Engine.Character|GetMesh _asbp_character)))

(fn CalculateDamage
  (bind _returnvalue (Game|GetPlayerCharacter 0))
  (bind _returnvalue_2 (Actor|GetComponentbyClass _returnvalue "/Game/Skilltree/AC_Skills.AC_Skills_C"))
  (bind (_rank _returnvalue_3 _skillout) (Default|QuerySkill _returnvalue_2 "/Game/Skilltree/Data/SwordDamage2.SwordDamage2"))
  (bind (_rank_2 _returnvalue_4 _skillout_2) (Default|QuerySkill _returnvalue_2 "/Game/Skilltree/Data/SwordDamage3.SwordDamage3"))
  (bind (_rank_3 _returnvalue_5 _skillout_3) (Default|QuerySkill _returnvalue_2 "/Game/Skilltree/Data/SwordDamage1.SwordDamage1"))
  (bind _values (Variables|/Game/Skilltree/Data/DA_Skill.DA_Skill_C|GetValues _skillout_2))
  (bind _values_2 (Variables|/Game/Skilltree/Data/DA_Skill.DA_Skill_C|GetValues _skillout_3))
  (bind _values_3 (Variables|/Game/Skilltree/Data/DA_Skill.DA_Skill_C|GetValues _skillout))
  (bind (_value _returnvalue_6) (Utilities|Map|Find _values_3 _rank))
  (bind (_value_2 _returnvalue_7) (Utilities|Map|Find _values _rank_2))
  (bind (_value_3 _returnvalue_8) (Utilities|Map|Find _values_2 _rank_3))
  (return (+ (Variables|Default|GetPlayerDamage) (Math|Float|SelectFloat _value_3 0.0 _returnvalue_8) (Math|Float|SelectFloat _value 0.0 _returnvalue_6) (Math|Float|SelectFloat _value_2 0.0 _returnvalue_7))))