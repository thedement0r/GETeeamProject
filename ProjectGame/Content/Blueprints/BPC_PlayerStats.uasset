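; Actor component that tracks current and maximum health for the player, dummy or AI that owns it.
; One tick after BeginPlay it casts the owner to identify its type, caches it and initializes health display on the HUD or health bar widget.
; DecreaseHealth updates the display and returns whether health is depleted.
; IncreaseHealth clamps to maximum; it and IncreaseMaxHealth refresh only the player's HUD bar.
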(event EventBeginPlay
  (Utilities|FlowControl|DelayUntilNextTick)
  (bind _asbp_third_person_character (Utilities|Casting|CastToBP_ThirdPersonCharacter (Components|GetOwner))
    (:then
      (Variables|Default|SetPlayer%20Character%20BP _asbp_third_person_character)
      (Variables|Default|SetisPlayer true))
    (:CastFailed
      (bind _asbp_dummy (Utilities|Casting|CastToBP_Dummy (Components|GetOwner))
        (:then
          (Variables|Default|SetDummyBP _asbp_dummy))
        (:CastFailed
          (bind _asbp_ai (Utilities|Casting|CastToBP_AI (Components|GetOwner)))
          (Variables|Default|SetAI_BP _asbp_ai)))
      (Variables|Default|SetisPlayer false)))
  (Progress|SetPercent (select (Variables|Default|GetisPlayer) (Variables|/Game/UI/WB_HUD.WB_HUD_C|GetHPBar (Variables|/Game/ThirdPerson/Blueprints/BP_ThirdPersonCharacter.BP_ThirdPersonCharacter_C|GetHUD%20Widget (Variables|Default|GetPlayer%20Character%20BP))) (Variables|/Game/UI/WB_DummyHealthBar.WB_DummyHealthBar_C|GetHealthBar (Variables|/Game/Blueprints/BP_Dummy.BP_Dummy_C|GetHealthBarUI (Variables|Default|GetDummyBP)))) (/ (Variables|Health|GetCurrent%20Health) (Variables|Health|GetMax%20Health)))
  (Rendering|Components|TextRender|SetText (select (Variables|Default|GetisPlayer) 0 (Variables|/Game/UI/WB_DummyHealthBar.WB_DummyHealthBar_C|GetHealthText (Variables|/Game/Blueprints/BP_Dummy.BP_Dummy_C|GetHealthBarUI (Variables|Default|GetDummyBP)))) (Utilities|Text|ToText(Float) (Variables|Health|GetCurrent%20Health) "HalfToEven")))

(event EventTick
  (params (DeltaSeconds :type Float%20%28single-precision%29)))

(fn DecreaseHealth
  (params (Damage :type Float%20%28double-precision%29))
  (if (not (<= (Variables|Health|GetCurrent%20Health) 0.0))
    (bind _output_get (Variables|Health|SetCurrent%20Health (- (Variables|Health|GetCurrent%20Health) Damage)))
    (Progress|SetPercent (select (Variables|Default|GetisPlayer) (Variables|/Game/UI/WB_HUD.WB_HUD_C|GetHPBar (Variables|/Game/ThirdPerson/Blueprints/BP_ThirdPersonCharacter.BP_ThirdPersonCharacter_C|GetHUD%20Widget (Variables|Default|GetPlayer%20Character%20BP))) (Variables|/Game/UI/WB_DummyHealthBar.WB_DummyHealthBar_C|GetHealthBar (Variables|/Game/Blueprints/BP_Dummy.BP_Dummy_C|GetHealthBarUI (Variables|Default|GetDummyBP)))) (/ _output_get (Variables|Health|GetMax%20Health)))
    (Rendering|Components|TextRender|SetText (select (Variables|Default|GetisPlayer) 0 (Variables|/Game/UI/WB_DummyHealthBar.WB_DummyHealthBar_C|GetHealthText (Variables|/Game/Blueprints/BP_Dummy.BP_Dummy_C|GetHealthBarUI (Variables|Default|GetDummyBP)))) (Utilities|Text|ToText(Float) (Variables|Health|GetCurrent%20Health) "HalfToEven"))
    (if (<= (Variables|Health|GetCurrent%20Health) 0.0)
      _
      (else
        (return false))))
  (return true))

(fn IncreaseMaxHealth
  (params (Health%20Incremetion :type Float%20%28double-precision%29))
  (Variables|Health|SetMax%20Health (+ (Variables|Health|GetMax%20Health) Health%20Incremetion))
  (Progress|SetPercent (Variables|/Game/UI/WB_HUD.WB_HUD_C|GetHPBar (Variables|/Game/ThirdPerson/Blueprints/BP_ThirdPersonCharacter.BP_ThirdPersonCharacter_C|GetHUD%20Widget (Variables|Default|GetPlayer%20Character%20BP))) (/ (Variables|Health|GetCurrent%20Health) (Variables|Health|GetMax%20Health))))

(fn IncreaseHealth
  (params (Added%20Health :type Float%20%28double-precision%29))
  (Variables|Health|SetCurrent%20Health (+ (Variables|Health|GetCurrent%20Health) Added%20Health))
  (if (> (Variables|Health|GetCurrent%20Health) (Variables|Health|GetMax%20Health))
    (Variables|Health|SetCurrent%20Health (Variables|Health|GetMax%20Health)))
  (Progress|SetPercent (Variables|/Game/UI/WB_HUD.WB_HUD_C|GetHPBar (Variables|/Game/ThirdPerson/Blueprints/BP_ThirdPersonCharacter.BP_ThirdPersonCharacter_C|GetHUD%20Widget (Variables|Default|GetPlayer%20Character%20BP))) (/ (Variables|Health|GetCurrent%20Health) (Variables|Health|GetMax%20Health))))