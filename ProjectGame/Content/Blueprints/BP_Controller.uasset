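; BP_Controller is a controller Blueprint that handles basic player movement, camera look and jumping.
; Legacy axis mappings move the controlled pawn along its root component's forward and right vectors and feed its yaw and pitch input.
; The Jump action calls Jump on player character 0 when pressed.
; BeginPlay also adds the default Enhanced Input mapping context, though every input event here uses legacy mappings.
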(event EventBeginPlay
  ;[1 1 1] In case we need enchanced input
  (Input|AddMappingContext (PlayerController|LocalPlayerSubsystems|GetEnhancedInputLocalPlayerSubsystem (Game|GetPlayerController 0)) "/Game/Template/ThirdPerson/IMC_Default.IMC_Default" 0 "(bIgnoreAllPressedKeysUntilRelease=True,bForceImmediately=False,bNotifyUserSettings=False)"))

(event Input|ActionEvents|InputActionJump
  (params (Key :type Key%20Structure :default "None"))
  ;[1 1 1] Action Mapping
  (:Pressed
    (Character|Jump (Game|GetPlayerCharacter 0))))

(event Input|AxisEvents|InputAxisTurn
  (params (AxisValue :type Float%20%28single-precision%29))
  ;[1 1 1] Camera
  (Pawn|Input|AddControllerYawInput (Pawn|GetControlledPawn) AxisValue))

(event Input|AxisEvents|InputAxisLookUp
  (params (AxisValue :type Float%20%28single-precision%29))
  ;[1 1 1] Camera
  (Pawn|Input|AddControllerPitchInput (Pawn|GetControlledPawn) AxisValue))

(event Input|AxisEvents|InputAxisMoveForward
  (params (AxisValue :type Float%20%28single-precision%29))
  (bind _returnvalue (Pawn|GetControlledPawn))
  ;[1 1 1] Movement
  (Pawn|Input|AddMovementInput _returnvalue (Math|Vector|GetForwardVector (Variables|/Script/Engine.Actor|GetRootComponent _returnvalue)) AxisValue false))

(event Input|AxisEvents|InputAxisMoveRight
  (params (AxisValue :type Float%20%28single-precision%29))
  (bind _returnvalue (Pawn|GetControlledPawn))
  ;[1 1 1] Movement
  (Pawn|Input|AddMovementInput _returnvalue (Math|Vector|GetRightVector (Variables|/Script/Engine.Actor|GetRootComponent _returnvalue)) AxisValue false))

(fn ConstructionScript)