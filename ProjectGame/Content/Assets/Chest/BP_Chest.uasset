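; BP_Chest is a lootable chest that rewards the player with an item and XP.
; On BeginPlay it spawns a BP_CombinationLock attached to the chest mesh and copies its unlocked state once into MinigameCompleted.
; OpenChest instead checks the player character's GameDone flag, then opens only once, playing the animation, notifying the quest component, granting XP and returning the item.
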(event EventBeginPlay
  (bind _returnvalue (Game|SpawnActorfromClass "/Game/Minigame/MinigameBP/BP_CombinationLock.BP_CombinationLock_C" (Math|Transform|MakeTransform "0, 0, 0" "0, 0, 0" "1.000000,1.000000,1.000000") "Undefined" "MultiplyWithRoot" 0 0))
  (Transformation|AttachComponentToComponent (Variables|/Script/Engine.Actor|GetRootComponent _returnvalue) (Variables|Default|GetChest) "None" "KeepRelative" "KeepRelative" "KeepRelative" true)
  (Variables|Default|SetMinigameCompleted (Variables|/Game/Minigame/MinigameBP/BP_CombinationLock.BP_CombinationLock_C|GetisUnlocked _returnvalue)))

(fn ConstructionScript)

(fn OpenChest
  (bind _asbp_character (Utilities|Casting|CastToBP_Character (Game|GetPlayerCharacter 0)))
  (if (and (not (Variables|Default|GetChestOpened)) (Variables|/Game/Blueprints/BP_Character.BP_Character_C|GetgameDone _asbp_character))
    (Variables|Default|SetChestOpened true)
    (Components|Animation|PlayAnimation (Variables|Default|GetChest) "/Game/Assets/Chest/Chest_Open.Chest_Open" false)
    (bind _asbp_character_2 (Utilities|Casting|CastToBP_Character (Game|GetPlayerCharacter 0)))
    (Default|OpenChest (Variables|/Game/Blueprints/BP_Character.BP_Character_C|GetBPC_Quest _asbp_character_2) self)
    (Default|IncreaseXP (Variables|/Game/Blueprints/BP_Character.BP_Character_C|GetBP_PlayerStats _asbp_character_2) (Variables|Default|GetAdded%20XP))
    (return (Variables|Default|GetItem))))