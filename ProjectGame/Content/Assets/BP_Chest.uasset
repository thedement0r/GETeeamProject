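; BP_Chest is a one-time openable loot chest that grants an item and experience to the player.
; OpenChest checks a ChestOpened flag, sets it, and plays the open animation without looping.
; It then casts the player pawn to BP_Character, notifies its quest component, adds XP to its stats component, and returns the Item.
; The event graph and construction script contain no logic.
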(event EventBeginPlay)

(event Collision|EventActorBeginOverlap
  (params (OtherActor :type Actor%20Object%20Reference)))

(event EventTick
  (params (DeltaSeconds :type Float%20%28single-precision%29)))

(fn ConstructionScript)

(fn OpenChest
  (if (not (Variables|Default|GetChestOpened))
    (Variables|Default|SetChestOpened true)
    (Components|Animation|PlayAnimation (Variables|Default|GetChest) "/Game/Assets/Chest_Open.Chest_Open" false)
    (bind _asbp_character (Utilities|Casting|CastToBP_Character (Game|GetPlayerCharacter 0)))
    (Default|OpenChest (Variables|/Game/Blueprints/BP_Character.BP_Character_C|GetBPC_Quest _asbp_character) self)
    (Default|IncreaseXP (Variables|/Game/Blueprints/BP_Character.BP_Character_C|GetBP_PlayerStats _asbp_character) (Variables|Default|GetAdded%20XP))
    (return (Variables|Default|GetItem))))