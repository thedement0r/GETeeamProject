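; BP_WhiteClover is an interactable white clover object that highlights itself through custom depth rendering when the player approaches.
; Player character overlap with its Sphere enables Render Custom Depth on three static meshes.
; End overlap also sets the flag to true, so the custom depth stays on after the player leaves.
; The construction script only calls the parent's.
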(event OnComponentEndOverlap(Sphere)
  (params (OverlappedComponent :type Primitive%20Component%20Object%20Reference) (OtherActor :type Actor%20Object%20Reference) (OtherComp :type Primitive%20Component%20Object%20Reference) (OtherBodyIndex :type Integer))
  (if (== (Game|GetPlayerCharacter 0) OtherActor)
    (Rendering|SetRenderCustomDepth (Variables|Default|GetStaticMesh) true)))

(event OnComponentBeginOverlap(Sphere)
  (params (OverlappedComponent :type Primitive%20Component%20Object%20Reference) (OtherActor :type Actor%20Object%20Reference) (OtherComp :type Primitive%20Component%20Object%20Reference) (OtherBodyIndex :type Integer) (bFromSweep :type Boolean) (SweepResult :type Hit%20Result%20Structure%20%28by%20ref%29))
  (if (== OtherActor (Game|GetPlayerCharacter 0))
    (Rendering|SetRenderCustomDepth (Variables|Default|GetStaticMesh) true)))

(fn ConstructionScript
  (|CallParentFunction))