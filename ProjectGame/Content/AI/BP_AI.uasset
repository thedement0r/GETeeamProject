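; Melee enemy character that fights with sword combos and can be stealth-assassinated by the player.
; A behavior-tree-called attack starts chained montages, with timer-looped sword traces and a separate sphere trace damaging tagged actors.
; Damage plays random hit reactions, cancels combos and knocks it back; death ragdolls it, updating player quest and XP.
; Camera-facing widgets show health and an assassination prompt; stealth kills play a victim montage, delay ragdoll and return alignment transforms.
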(event OnComponentBeginOverlap(AssassinationRadius)
  (params (OverlappedComponent :type Primitive%20Component%20Object%20Reference) (OtherActor :type Actor%20Object%20Reference) (OtherComp :type Primitive%20Component%20Object%20Reference) (OtherBodyIndex :type Integer) (bFromSweep :type Boolean) (SweepResult :type Hit%20Result%20Structure%20%28by%20ref%29))
  (Utilities|Casting|CastToBP_Character OtherActor)
  (Rendering|SetVisibility (Variables|Default|GetAssassinate%20Widget) true false))

(event OnComponentEndOverlap(AssassinationRadius)
  (params (OverlappedComponent :type Primitive%20Component%20Object%20Reference) (OtherActor :type Actor%20Object%20Reference) (OtherComp :type Primitive%20Component%20Object%20Reference) (OtherBodyIndex :type Integer))
  (Utilities|Casting|CastToBP_Character OtherActor)
  (Rendering|SetVisibility (Variables|Default|GetAssassinate%20Widget) false false))

(event Custom|Sword%20Attack
  ;[1 1 1] Combo system
  (if (Variables|Default|GetisAttacking)
    (Variables|Default|SetsaveAttack true)
    (else
      (Variables|Default|SetisAttacking true)
      (switch int (Variables|Default|GetAttackIndex)
        (:0
          (CallFunction|Attack1))
        (:1
          (CallFunction|Attack2))
        (:2
          (CallFunction|Attack4))))))

(event Custom|Sword%20Attack%20Combo
  ;[1 1 1] Combo system
  (if (Variables|Default|GetsaveAttack)
    (Variables|Default|SetsaveAttack false)
    (switch int (Variables|Default|GetAttackIndex)
      (:0
        (CallFunction|Attack1))
      (:1
        (CallFunction|Attack2))
      (:2
        (CallFunction|Attack4)))
    (else
      (CallFunction|StopCombo))))

(event Custom|Start%20Sword%20Trace
  ;[1 1 1] Sword Trace
  (bind _returnvalue (Utilities|Time|SetTimerbyEvent (delegate Custom|Sword%20Trace%20Loop) 0.01 true))
  (Variables|Default|SetSwordTraceLoop _returnvalue))

(event Custom|Sword%20Trace%20Loop
  ;[1 1 1] Sword Trace
  (bind (_outhit _returnvalue) (Collision|SphereTraceByChannel (Transformation|GetWorldLocation (Variables|Default|GetSword%20Top%20Point)) (Transformation|GetWorldLocation (Variables|Default|GetSword%20Bottom%20Point)) 12.0 "TraceTypeQuery1" false 0 "None" true "(R=1.000000,G=0.000000,B=0.000000,A=1.000000)" "(R=0.000000,G=1.000000,B=0.000000,A=1.000000)" 0.2))
  (if _returnvalue
    (if (and (Variables|Default|GetisAttacking) (Actor|ActorHasTag (.HitActor (Collision|BreakHitResult _outhit)) "abc"))
      (Utilities|FlowControl|DoOnce false :!label _label
        (:Completed
          (Game|Damage|ApplyDamage (.HitActor (Collision|BreakHitResult _outhit)) 1e+01 0 0)
          (Utilities|FlowControl|Delay 1.0)
          (goto _label Reset))))))

(event Custom|Stop%20Sword%20Trace
  ;[1 1 1] Sword Trace
  (Utilities|Time|ClearandInvalidateTimerbyHandle (Variables|Default|GetSwordTraceLoop)))

(event Custom|Sphere%20Trace
  (bind _sphere_trace_pos (Variables|Default|GetSphere%20Trace%20Pos))
  (bind _returnvalue (Transformation|GetWorldLocation _sphere_trace_pos))
  ;[1 1 1] Sphere Trace for stab+kick
  (bind (_outhit _returnvalue_2) (Collision|SphereTraceByChannel _returnvalue _returnvalue 25.0 "TraceTypeQuery1" false 0 "None"))
  (if _returnvalue_2
    (if (and (Variables|Default|GetisAttacking) (Actor|ActorHasTag (.HitActor (Collision|BreakHitResult _outhit)) "abc"))
      (Game|Damage|ApplyDamage (.HitActor (Collision|BreakHitResult _outhit)) 1e+01 0 0))))

(event Custom|Stop%20Combo
  ;[1 1 1] Combo system
  (Variables|Default|SetisAttacking false)
  (Variables|Default|SetAttackIndex 0))

(event Custom|Attack%204
  ;[1 1 1] Combo system
  (Utilities|FlowControl|DoOnce false :!label _label
    (:Completed
      (Utilities|FlowControl|Delay 0.1)
      (Animation|Montage|PlayMontage (Variables|Character|GetMesh) "/Game/Animations/SwordAttack/Attack3_Montage.Attack3_Montage"
        (:then
          (Variables|Default|SetAttackIndex 4)
          (goto _label Reset))))))

(event Custom|Attack%201
  ;[1 1 1] Combo system
  (Utilities|FlowControl|DoOnce false :!label _label
    (:Completed
      (Utilities|FlowControl|Delay 0.1)
      (Animation|Montage|PlayMontage (Variables|Character|GetMesh) "/Game/Animations/SwordAttack/Attack1_Montage.Attack1_Montage"
        (:then
          (Variables|Default|SetAttackIndex 1)
          (goto _label Reset))))))

(event Custom|Ragdoll
  ;[1 1 1] Ragdoll
  (Utilities|FlowControl|Delay 2.5)
  (Physics|SetSimulatePhysics (Variables|Character|GetMesh) true))

(event Custom|Attack2
  ;[1 1 1] Combo system
  (Utilities|FlowControl|DoOnce false :!label _label
    (:Completed
      (Utilities|FlowControl|Delay 0.1)
      (Animation|Montage|PlayMontage (Variables|Character|GetMesh) "/Game/Animations/SwordAttack/Attack2_Montage.Attack2_Montage"
        (:then
          (Variables|Default|SetAttackIndex 2)
          (goto _label Reset))))))

(event Custom|SwordAttackCombpCallFromBT
  ;[1 1 1] Combo system
  (if (Variables|Default|GetcanAttack)
    (CallFunction|SwordAttack)))

(event Custom|Attack%203
  ;[1 1 1] Combo system
  ;;[1 1 1] Not using for AI
  (Utilities|FlowControl|DoOnce false :!label _label
    (:Completed
      (Utilities|FlowControl|Delay 0.1)
      (Animation|Montage|PlayMontage (Variables|Character|GetMesh) "/Game/Animations/SwordAttack/Kick_Montage.Kick_Montage"
        (:then
          (Variables|Default|SetAttackIndex 3)
          (goto _label Reset))))))

(event EventTick
  (params (DeltaSeconds :type Float%20%28single-precision%29))
  (Transformation|SetWorldRotation (Variables|Default|GetAssassinate%20Widget) (Math|Rotator|FindLookatRotation (Transformation|GetWorldLocation (Variables|Default|GetAssassinate%20Widget)) (Transformation|GetWorldLocation (Variables|/Script/Engine.PlayerCameraManager|GetTransformComponent (Game|GetPlayerCameraManager 0)))) false false))

(event EventBeginPlay
  (bind _aswb_dummy_health_bar (Utilities|Casting|CastToWB_DummyHealthBar (UserInterface|GetWidget (Variables|Default|GetHealth%20Bar%20Widget))))
  (Variables|Default|SetHealthBar%20UI _aswb_dummy_health_bar))

(event Game|Damage|EventAnyDamage
  (params (Damage :type Float%20%28single-precision%29) (DamageType :type Damage%20Type%20Object%20Reference) (InstigatedBy :type Controller%20Object%20Reference) (DamageCauser :type Actor%20Object%20Reference))
  (if (not (Variables|Default|GetisDead))
    (Animation|PlayAnimMontage (Utilities|Array|Get(acopy) (Variables|Default|GethitAnims) (Math|Random|RandomIntegerinRange 0 (- (Utilities|Array|Length (Variables|Default|GethitAnims)) 1))) 1.0 "None")
    (CallFunction|StopCombo)
    (bind _asbp_character (Utilities|Casting|CastToBP_Character (Game|GetPlayerCharacter 0)))
    (Character|LaunchCharacter (* (Math|Vector|GetForwardVector (Transformation|GetActorRotation _asbp_character)) 7e+02) false false)
    (bind _isplayerdead (Default|DecreaseHP (Variables|Default|GetBP_PlayerStats) Damage))
    (if _isplayerdead
      (Collision|SetCollisionObjectType (Variables|Character|GetMesh) "ECC_PhysicsBody")
      (Physics|SetSimulatePhysics (Variables|Character|GetMesh) true)
      (Rendering|SetVisibility (Variables|Default|GetHealth%20Bar%20Widget) false false)
      (Variables|Default|SetisDead true)
      (Variables|Default|SetcanAttack false)
      (Utilities|FlowControl|DoOnce false
        (:Completed
          (bind _asbp_character_2 (Utilities|Casting|CastToBP_Character (Game|GetPlayerCharacter 0)))
          (Default|EliminateEnemy (Variables|/Game/Blueprints/BP_Character.BP_Character_C|GetBPC_Quest _asbp_character_2) self)
          (Pawn|Components|CharacterMovement|SetMovementMode (Variables|Character|GetCharacterMovement) "MOVE_None" 0)
          (Default|IncreaseXP (Variables|/Game/Blueprints/BP_Character.BP_Character_C|GetBP_PlayerStats _asbp_character_2) (Variables|Default|GetAdded%20XP))
          (Development|PrintString (Utilities|GetDisplayName (Variables|/Game/Blueprints/BP_Character.BP_Character_C|GetBP_PlayerStats _asbp_character_2))))))))

(fn ConstructionScript)

(fn Attack
  (CallFunction|SwordAttackCombpCallfromBT)
  (return 0.4))

(fn StealthBackAssassin
  (if (not (Variables|Default|GetisDead))
    (Variables|Default|SetisDead true)
    (Animation|PlayAnimMontage "/Game/Animations/Assassination/Paired_Knife_Stealth_KidneyAndNeck_Vic_Montage.Paired_Knife_Stealth_KidneyAndNeck_Vic_Montage" 1.0 "None")
    (CallFunction|Ragdoll)
    (Rendering|SetVisibility (Variables|Default|GetAssassinate%20Widget) false false)
    (Pawn|Components|CharacterMovement|SetMovementMode (Variables|Character|GetCharacterMovement) "MOVE_None" 0)
    (return (Transformation|GetWorldLocation (Variables|Default|GetAssassin%20REF)) (Transformation|GetActorRotation))))