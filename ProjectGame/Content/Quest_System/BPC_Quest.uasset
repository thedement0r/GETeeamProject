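; BPC_Quest is a quest component that tracks one active quest and its objectives, displaying them on a quest HUD widget it creates at BeginPlay.
; Eliminate-enemy, open-chest and pick-item events match against the quest's objectives, mark them completed and update the HUD.
; Enemy kills drain a working array seeded from the objective's target actors.
; A completion counter clears the quest and plays the completion animation once it reaches the objective count.
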(event Custom|Set%20Active%20Quest%20Text
  (Rendering|Components|TextRender|SetText (Variables|/Game/Quest_System/WB_QuestHUD.WB_QuestHUD_C|GetActiveQuestText (Variables|Default|GetQuest%20HUD%20Widget)) (Utilities|Text|ToText(String) (.Name (Utilities|Struct|BreakS_Quest (Variables|Default|GetactiveQuest)))))
  (Default|ShowQuestPanel (Variables|Default|GetQuest%20HUD%20Widget)))

(event Custom|Set%20Objectives
  (Default|FillObjectives (Variables|Default|GetQuest%20HUD%20Widget) (.objectives (Variables|Default|GetactiveQuest))))

(event Custom|Eliminate%20enemy
  (params (Enemy%20Eliminated :type Actor%20Object%20Reference))
  (for _array_element (.objectives (Variables|Default|GetactiveQuest))
    (if (and (not (.Completed (Utilities|Struct|BreakS_QuestObjective _array_element))) (.IsEliminateEnemyObject (Utilities|Struct|BreakS_QuestObjective _array_element)))
      (if (!= (Utilities|Array|Length (Variables|Default|GetEnemy%20Actors%20Array)) 0)
        _
        (else
          (bind _output_get (Variables|Default|SetEnemy%20Actors%20Array (.ActorsToEliminate (Utilities|Struct|BreakS_QuestObjective _array_element))))))
      (Utilities|Array|RemoveItem _output_get Enemy%20Eliminated)
      (|SetBy-RefVar _array_element (Utilities|Struct|MakeS_QuestObjective (.NameAim (Utilities|Struct|BreakS_QuestObjective _array_element)) false (.ActorsToEliminate (Utilities|Struct|BreakS_QuestObjective _array_element)) (.IsEliminateEnemyObject (Utilities|Struct|BreakS_QuestObjective _array_element)) false 0 0 false))
      (Development|PrintString (Utilities|String|ToString(Integer) (Utilities|Array|Length (Variables|Default|GetEnemy%20Actors%20Array))))
      (if (== (Utilities|Array|Length (Variables|Default|GetEnemy%20Actors%20Array)) 0)
        (|SetBy-RefVar _array_element (Utilities|Struct|MakeS_QuestObjective (.NameAim (Utilities|Struct|BreakS_QuestObjective _array_element)) true 0 (.IsEliminateEnemyObject (Utilities|Struct|BreakS_QuestObjective _array_element)) false 0 0 false))
        (Default|CompleteObjective (Variables|Default|GetQuest%20HUD%20Widget) _array_element)
        (CallFunction|ObjectiveCompleted)))))

(event Custom|Pick%20Item
  (params (Item :type Actor%20Object%20Reference))
  (for _array_element (.objectives (Variables|Default|GetactiveQuest))
    (if (and (.IsItemObject (Utilities|Struct|BreakS_QuestObjective _array_element)) (== Item (.Itemstopick (Utilities|Struct|BreakS_QuestObjective _array_element))))
      (|SetBy-RefVar _array_element (Utilities|Struct|MakeS_QuestObjective (.NameAim (Utilities|Struct|BreakS_QuestObjective _array_element)) true (.ActorsToEliminate (Utilities|Struct|BreakS_QuestObjective _array_element)) (.IsEliminateEnemyObject (Utilities|Struct|BreakS_QuestObjective _array_element)) (.IsItemObject (Utilities|Struct|BreakS_QuestObjective _array_element)) 0 0 false))
      (Default|CompleteObjective (Variables|Default|GetQuest%20HUD%20Widget) _array_element)
      (CallFunction|ObjectiveCompleted)
      (Development|PrintString "DONE"))))

(event Custom|Objective%20Completed
  (Math|Integer|IncrementInt (Variables|Default|Getobjectives%20completed)
    (:%20%20
      (if (>= (Variables|Default|Getobjectives%20completed) (Utilities|Array|Length (.objectives (Variables|Default|GetactiveQuest))))
        (Development|PrintString "Quest Completed")
        (Variables|Default|SetactiveQuest "")
        (Variables|Default|Setobjectives%20completed 0)
        (Default|PlayQuestCompletedAnim (Variables|Default|GetQuest%20HUD%20Widget))))))

(event Custom|Open%20Chest
  (params (Chest :type Actor%20Object%20Reference))
  (for _array_element (.objectives (Variables|Default|GetactiveQuest))
    (if (and (== Chest (.Chesttoopen (Utilities|Struct|BreakS_QuestObjective _array_element))) (.IsChestObjective (Utilities|Struct|BreakS_QuestObjective _array_element)))
      (|SetBy-RefVar _array_element (Utilities|Struct|MakeS_QuestObjective (.NameAim (Utilities|Struct|BreakS_QuestObjective _array_element)) true (.ActorsToEliminate (Utilities|Struct|BreakS_QuestObjective _array_element)) false false 0 0 (.IsChestObjective (Utilities|Struct|BreakS_QuestObjective _array_element))))
      (Default|CompleteObjective (Variables|Default|GetQuest%20HUD%20Widget))
      (CallFunction|ObjectiveCompleted))))

(event EventBeginPlay
  (bind _returnvalue (UserInterface|CreateWidget "/Game/Quest_System/WB_QuestHUD.WB_QuestHUD_C"))
  (bind _output_get (Variables|Default|SetQuest%20HUD%20Widget _returnvalue))
  (UserInterface|Viewport|AddtoViewport _output_get 0)
  (Default|HideQuestPanel (Variables|Default|GetQuest%20HUD%20Widget)))