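; Crafting component that toggles the crafting menu and tracks which craftable items are unlocked by level.
; IA_Crafting lazily creates WB_CraftingMenu, switches input mode and cursor, and refreshes slots from DT_CraftablePlayerItems and the unlocked list.
; InitCalculateCraft reads a given data table's rows, async-loads valid item classes not yet unlocked, and unlocks those whose required level is zero or reached.
; It then prints the unlocked list for debugging.
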(event Custom|InitCalculateCraft
  (params (Datatable%20to%20use :type Data%20Table%20Object%20Reference))
  (Variables|Default|SetDatatable%20To%20Use Datatable%20to%20use)
  (bind _outrownames (DataTable|GetDataTableRowNames (Variables|Default|GetDatatable%20To%20Use)))
  (Variables|Default|SetAll%20Craftable%20Items _outrownames)
  (CallFunction|CalculateUnlockedItems)
  ;[1 1 1] debug
  (CallFunction|PrintUnlockedItems))

(event Custom|LoadAsync
  (params (NewParam :type A%20Master%20Pick%20Up%20Soft%20Class%20Reference))
  (Utilities|AsyncLoadClassAsset NewParam))

(event Input|EnhancedActionEvents|EnhancedInputActionIA_Crafting
  (params (ActionValue :type Boolean) (ElapsedSeconds :type Float%20%28double-precision%29) (TriggeredSeconds :type Float%20%28double-precision%29) (InputAction :type Input%20Action%20Object%20Reference :default "/Game/Crafting/IA_Crafting.IA_Crafting"))
  (bind _returnvalue (Game|GetPlayerController 0))
  (bind _returnvalue_2 (Game|GetPlayerController 0))
  (:Completed
    (Utilities|IsValid (Variables|Default|GetCraftingMenuREF)
      (:Is%20Valid
        (if (Widget|IsVisible (Variables|Default|GetCraftingMenuREF))
          (Widget|SetVisibility (Variables|Default|GetCraftingMenuREF) "Hidden")
          (Input|SetInputModeGameOnly _returnvalue_2 false)
          (Variables|/Script/Engine.PlayerController|SetbShowMouseCursor _returnvalue_2 false)
          (else
            (UserInterface|Viewport|AddtoViewport (stale _output_get) 0 :!label _label)
            (Input|SetInputModeGameandUI _returnvalue (Variables|Default|GetCraftingMenuREF) "DoNotLock" true false)
            (Variables|/Script/Engine.PlayerController|SetbShowMouseCursor _returnvalue true)
            (Default|UpdateAllCraftingSlots (Variables|Default|GetCraftingMenuREF) "/Game/Crafting/DT_CraftablePlayerItems.DT_CraftablePlayerItems" (Variables|Default|GetUnlocked%20Craftable%20Items) "NewEnumerator0")
            (Widget|SetVisibility (Variables|Default|GetCraftingMenuREF) "Visible")
            (Default|HideIngridients (Variables|Default|GetCraftingMenuREF)))))
      (:Is%20Not%20Valid
        (bind _returnvalue_3 (UserInterface|CreateWidget "/Game/Crafting/WB_CraftingMenu.WB_CraftingMenu_C"))
        (bind _output_get (Variables|Default|SetCraftingMenuREF _returnvalue_3))
        (goto _label)))))

(fn CalculateUnlockedItems
  (for _array_element (Variables|Default|GetAll%20Craftable%20Items)
    (LocalVariables|SetCurrent%20Array%20Element _array_element)
    (if (not (Utilities|Array|ContainsItem (Variables|Default|GetUnlocked%20Craftable%20Items) (LocalVariables|GetCurrent%20Array%20Element)))
      (bind _out_row (CallFunction|GetCraftableItemfromName (LocalVariables|GetCurrent%20Array%20Element)))
      (LocalVariables|SetCurrent%20Item%20Row _out_row)
      (if (Utilities|IsValidClass (Utilities|ResolveSoftReference (.CraftingItem (Utilities|Struct|BreakS_CraftableItem (LocalVariables|GetCurrent%20Item%20Row)))))
        (CallFunction|LoadAsync (.CraftingItem (Utilities|Struct|BreakS_CraftableItem (LocalVariables|GetCurrent%20Item%20Row))))
        (if (== (.RequiredLvl (Utilities|Struct|BreakS_CraftableItem (LocalVariables|GetCurrent%20Item%20Row))) 0)
          (Utilities|Array|Add (Variables|Default|GetUnlocked%20Craftable%20Items) (LocalVariables|GetCurrent%20Array%20Element) :!label _label)
          (elif (>= (Variables|Default|GetCurrentLevel) (.RequiredLvl (Utilities|Struct|BreakS_CraftableItem (LocalVariables|GetCurrent%20Item%20Row))))
            (goto _label)))))))

(fn GetCraftableItemfromName
  (params (Row%20Name :type Name))
  (bind _returnvalue (Class|DataTableFunctionLibrary|DoesDataTableRowExist (Variables|Default|GetDatatable%20To%20Use) Row%20Name))
  (if _returnvalue
    (bind _returnvalue_2 (Utilities|GetDataTableRow (Variables|Default|GetDatatable%20To%20Use) Row%20Name)
      (:then
        (return _returnvalue_2)))))

(fn PrintUnlockedItems
  (for _array_element (Variables|Default|GetUnlocked%20Craftable%20Items)
    (Development|PrintString (Utilities|String|ToString(Name) _array_element))))